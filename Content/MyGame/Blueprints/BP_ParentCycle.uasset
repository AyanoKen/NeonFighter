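; BP_ParentCycle is a player-driven cycle, named as a parent class, with throttle, brake, steering and camera yaw through Enhanced Input.
; Tick ramps speed up, brakes or coasts down within limits, then applies a swept forward offset without delta-time scaling.
; Steering yaws the actor and leans the mesh within a clamp, levelling it on release.
; The capsule hit event is empty, and a speed reset sits unconnected.
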(event `EnhancedInput|/Game/VehicleTemplate/Input/Actions/IA_Throttle`
  (params (ActionValue :type "Float (double-precision)") (ElapsedSeconds :type "Float (double-precision)") (TriggeredSeconds :type "Float (double-precision)") (InputAction :type "InputAction Object Reference" :default "/Game/VehicleTemplate/Input/Actions/IA_Throttle.IA_Throttle"))
  (:`Started`
    (set `self.IsAccelerating` true))
  (:`Completed`
    (set `self.IsAccelerating` false)))

(event `self.ReceiveBeginPlay`
  (set `self.Instigator` null))

(event `self.ReceiveTick`
  (params (DeltaSeconds :type "Float (single-precision)"))
  (`|ExecutionSequence`
    (:`then_0`
      (if (`self.IsAccelerating`)
        (set `self.CurrentSpeed` (`KismetMathLibrary.FClamp` (+ (`self.CurrentSpeed`) (* (`self.Acceleration`) DeltaSeconds)) 0.0 (`self.MaxSpeed`)))
        (elif (`self.IsBraking`)
          (set `self.CurrentSpeed` (`KismetMathLibrary.FClamp` (- (`self.CurrentSpeed`) (* DeltaSeconds (`self.BrakeForce`))) 0.0 (`self.MaxSpeed`)))
          (else
            (set `self.CurrentSpeed` (`KismetMathLibrary.FClamp` (- (`self.CurrentSpeed`) (* DeltaSeconds (`self.FallOffSpeed`))) 0.0 (`self.MaxSpeed`)))))))
    (:`then_1`
      (`self.K2_AddActorWorldOffset` (* (`SceneComponent.GetForwardVector` (`self.StaticMesh`)) (`self.CurrentSpeed`)) true))))

(event `EnhancedInput|/Game/VehicleTemplate/Input/Actions/IA_LookAround`
  (params (ActionValue :type "Float (double-precision)") (ElapsedSeconds :type "Float (double-precision)") (TriggeredSeconds :type "Float (double-precision)") (InputAction :type "InputAction Object Reference" :default "/Game/VehicleTemplate/Input/Actions/IA_LookAround.IA_LookAround"))
  (:`Triggered`
    (`SceneComponent.K2_AddLocalRotation` (`self.SpringArm`) (`KismetMathLibrary.MakeRotator` 0.0 0.0 ActionValue) false false)))

(event `EnhancedInput|/Game/VehicleTemplate/Input/Actions/IA_Steering`
  (params (ActionValue :type "Float (double-precision)") (ElapsedSeconds :type "Float (double-precision)") (TriggeredSeconds :type "Float (double-precision)") (InputAction :type "InputAction Object Reference" :default "/Game/VehicleTemplate/Input/Actions/IA_Steering.IA_Steering"))
  (:`Triggered`
    (`self.K2_AddActorLocalRotation` (`KismetMathLibrary.MakeRotator` 0.0 0.0 (* ActionValue (`self.TurnSpeed`) (`GameplayStatics.GetWorldDeltaSeconds`))))
    (`SceneComponent.K2_SetRelativeRotation` (`self.StaticMesh`) (`KismetMathLibrary.MakeRotator` (`KismetMathLibrary.FClamp` (* ActionValue (`self.LeanAngle`)) -20.0 20.0)) false false))
  (:`Completed`
    (`SceneComponent.K2_SetRelativeRotation` (`self.StaticMesh`) (`KismetMathLibrary.MakeRotator` 0.0) false false)))

(event `EnhancedInput|/Game/VehicleTemplate/Input/Actions/IA_Brake`
  (params (ActionValue :type "Float (double-precision)") (ElapsedSeconds :type "Float (double-precision)") (TriggeredSeconds :type "Float (double-precision)") (InputAction :type "InputAction Object Reference" :default "/Game/VehicleTemplate/Input/Actions/IA_Brake.IA_Brake"))
  (:`Started`
    (set `self.IsBraking` true))
  (:`Completed`
    (set `self.IsBraking` false)))

(event `self.CapsuleComponent.OnComponentHit`
  (params (HitComponent :type "PrimitiveComponent Object Reference") (OtherActor :type "Actor Object Reference") (OtherComp :type "PrimitiveComponent Object Reference") (NormalImpulse :type "Vector Structure") (Hit :type "HitResult Structure (by ref)")))

(fn `UserConstructionScript`)