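; Light trail component that manages server-side spawning of trail collider segments for its owning pawn.
; On BeginPlay the authority pre-spawns a pool of deactivated colliders far below the pawn, each linked back to the component.
; Start and stop requests run on authority or route through server calls, toggling a looping SpawnSegment_Server timer whose target is absent here.
; An exhausted pool spawns unregistered extras; ReturnToPool and OnRep_TrailColor are empty.
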(event `self.ReceiveBeginPlay`
  (bind _output_get (set `self.OwnerPawn` (`self.GetOwner`)))
  (if (`Actor.HasAuthority` _output_get)
    (for _ (range (`self.PoolSize`))
      (bind _returnvalue (`|SpawnActorFromClass` (`self.ColliderClass`) (`KismetMathLibrary.Conv_VectorToTransform` (+ (`Actor.K2_GetActorLocation` (`self.OwnerPawn`)) (0.0 0.0 -10000.0))) "AlwaysSpawn" "MultiplyWithRoot" null null))
      (`/Game/MyGame/Blueprints/BP_TrailCollider.DeactiveSegment` _returnvalue)
      (`KismetArrayLibrary.Array_Add` (`self.SegmentPool`) _returnvalue)
      (set `/Game/MyGame/Blueprints/BP_TrailCollider.OwningManager` self _returnvalue))))

(event `RequestStartTrail`
  (if (`Actor.HasAuthority` (`self.OwnerPawn`))
    (`self.StartTrail_ServerLogic`)
    (else
      (`self.Server_StartTrail`))))

(event `RequestStopTrail`
  (if (`Actor.HasAuthority` (`self.OwnerPawn`))
    (`self.StopTrail_ServerLogic`)
    (else
      (`self.Server_StopTrail`))))

(event `Server_StartTrail`
  (`self.StartTrail_ServerLogic`))

(event `Server_StopTrail`
  (`self.StopTrail_ServerLogic`))

(event `StartTrail_ServerLogic`
  (set `self.IsSpawning?` true)
  (bind _returnvalue (`KismetSystemLibrary.K2_SetTimer` null "SpawnSegment_Server" (`self.SpawnInterval`) true))
  (set `self.SpawnTimerHandle` _returnvalue))

(event `StopTrail_ServerLogic`
  (set `self.IsSpawning?` false)
  (`KismetSystemLibrary.K2_ClearAndInvalidateTimerHandle` (`self.SpawnTimerHandle`)))

(fn `GetFreeSegmentFromPool`
  (returns (Segment :type "/Game/MyGame/Blueprints/BP_TrailCollider Object Reference"))
  (for _array_element (`self.SegmentPool`)
    (if (not (`/Game/MyGame/Blueprints/BP_TrailCollider.isActive?` _array_element))
      (return _array_element)))
  (bind _returnvalue (`|SpawnActorFromClass` (`self.ColliderClass`) (`KismetMathLibrary.Conv_VectorToTransform` (+ (`Actor.K2_GetActorLocation` (`self.OwnerPawn`)) (0.0 0.0 -10000.0))) "AlwaysSpawn" "MultiplyWithRoot" null null))
  (return _returnvalue))

(fn `OnRep_TrailColor`)

(fn `ReturnToPool`)