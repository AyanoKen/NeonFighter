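; BP_VisualTrail is a short-lived glowing trail actor that draws a spline mesh between two points.
; InitVisual sets the spline endpoints, creates a dynamic M_Glow material with the given color and emissive strength, unhides the actor and starts a lifetime timer.
; When the timer fires, FadeOutAndDestroy runs a timeline that lowers the material's opacity, then destroys the actor.
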(event `InitVisual`
  (params (Start :type "Vector Structure") (End :type "Vector Structure") (Color :type "LinearColor Structure") (Lifetime :type "Float (double-precision)"))
  (bind _splinemesh (`self.SplineMesh`))
  (set `self.TrailColor` Color)
  (set `self.LifeTime` Lifetime)
  (`SplineMeshComponent.SetStartAndEnd` _splinemesh Start (0.0 0.0 0.0) End (0.0 0.0 0.0) true)
  (bind _returnvalue (`PrimitiveComponent.CreateDynamicMaterialInstance` _splinemesh 0 "/Game/MyGame/Models/LightCycle1/M_Glow.M_Glow" "None"))
  (bind _output_get (set `self.DynamicMaterial` _returnvalue))
  (`MaterialInstanceDynamic.SetVectorParameterValue` _output_get "TrailColor" (`self.TrailColor`))
  (`MaterialInstanceDynamic.SetScalarParameterValue` _output_get "EmissiveStrength" 1.0)
  (`KismetSystemLibrary.K2_SetTimer` null "FadeOutAndDestroy" (`self.LifeTime`))
  (`self.SetActorHiddenInGame` false))

(event `FadeOutAndDestroy`
  (bind (_direction _alpha) (`Timeline|FadeTimeline`)
    (:`Update`
      (`MaterialInstanceDynamic.SetScalarParameterValue` (`self.DynamicMaterial`) "Opacity" (- 1.0 _alpha)))
    (:`Finished`
      (`self.K2_DestroyActor`))))

(fn `UserConstructionScript`)