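; Damaging trail segment collider that hurts any BP_ParentCycle touching it, except the bike that owns it.
; InitCollider centres a box between two points, aims its X axis along them, sets its Z extent from their distance and starts a lifetime timer.
; Server-side overlaps deal damage once, or on a shared looping timer when DamageInterval is positive.
; On expiry, ReturnToPool deactivates the collider, then destroys it despite its name.
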(event `InitCollider`
  (params (Start :type "Vector Structure") (End :type "Vector Structure") (OwnerBikeRef :type "Actor Object Reference") (Damage :type "Float (double-precision)") (Lifetime :type "Float (double-precision)"))
  (bind _returnvalue (- End Start))
  (bind _box (`self.Box`))
  (set `self.isActive?` true)
  (set `self.OwnerBike` OwnerBikeRef)
  (set `self.Damage` Damage)
  (set `self.LifeTime` Lifetime)
  (`SceneComponent.K2_SetWorldLocationAndRotation` _box (* (+ Start End) 0.5) (`KismetMathLibrary.MakeRotFromX` (`KismetMathLibrary.Normal` _returnvalue)) false false)
  (`BoxComponent.SetBoxExtent` _box (`KismetMathLibrary.MakeVector` 50.0 10.0 (* (`KismetMathLibrary.VSize` _returnvalue) 0.5)) true)
  (`KismetSystemLibrary.K2_SetTimer` null "ReturnToPool" (`self.LifeTime`))
  (`self.SetActorHiddenInGame` false)
  (`self.SetActorEnableCollision` true))

(event `self.Box.OnComponentBeginOverlap`
  (params (OverlappedComponent :type "PrimitiveComponent Object Reference") (OtherActor :type "Actor Object Reference") (OtherComp :type "PrimitiveComponent Object Reference") (OtherBodyIndex :type Integer) (bFromSweep :type Boolean) (SweepResult :type "HitResult Structure (by ref)"))
  (bind _overlappingactors (`self.OverlappingActors`))
  (if (and (`self.HasAuthority`) (`KismetSystemLibrary.IsValid` OtherActor))
    (cast `/Game/MyGame/Blueprints/BP_ParentCycle` OtherActor)
    (if (== OtherActor (`self.OwnerBike`))
      _
      (elif (<= (`self.DamageInterval`) 0.0)
        (`GameplayStatics.ApplyDamage` OtherActor (`self.Damage`) (`self.GetInstigatorController` (`self.OwnerBike`)) self "/Script/Engine.DamageType")
        (elif (not (`KismetArrayLibrary.Array_Contains` _overlappingactors OtherActor))
          (`KismetArrayLibrary.Array_Add` _overlappingactors OtherActor)
          (if (not (`KismetSystemLibrary.K2_IsValidTimerHandle` (`self.PeriodicDamageTimerHandle`)))
            (bind _returnvalue (`KismetSystemLibrary.K2_SetTimer` null "ApplyPeriodicDamage" (`self.DamageInterval`) true))
            (set `self.PeriodicDamageTimerHandle` _returnvalue)))))))

(event `self.Box.OnComponentEndOverlap`
  (params (OverlappedComponent :type "PrimitiveComponent Object Reference") (OtherActor :type "Actor Object Reference") (OtherComp :type "PrimitiveComponent Object Reference") (OtherBodyIndex :type Integer))
  (bind _overlappingactors (`self.OverlappingActors`))
  (if (and (`self.HasAuthority`) (`KismetSystemLibrary.IsValid` OtherActor))
    (if (`KismetArrayLibrary.Array_Contains` _overlappingactors OtherActor)
      (`KismetArrayLibrary.Array_RemoveItem` _overlappingactors OtherActor)
      (if (<= (`KismetArrayLibrary.Array_Length` _overlappingactors) 0)
        (`KismetSystemLibrary.K2_ClearAndInvalidateTimerHandle` (`self.PeriodicDamageTimerHandle`))))))

(fn `ApplyPeriodicDamage`
  (for _array_element (`self.OverlappingActors`)
    (if (`KismetSystemLibrary.IsValid` _array_element)
      (`GameplayStatics.ApplyDamage` _array_element (`self.Damage`) (`self.GetInstigatorController` (`self.OwnerBike`)) self "/Script/Engine.DamageType"))))

(fn `ReturnToPool`
  (set `self.isActive?` false)
  (`KismetArrayLibrary.Array_Clear` (`self.OverlappingActors`))
  (`KismetSystemLibrary.K2_ClearAndInvalidateTimerHandle` (`self.PeriodicDamageTimerHandle`))
  (`self.SetActorHiddenInGame` true)
  (`self.SetActorEnableCollision` false)
  (`self.K2_DestroyActor`))

(fn `UserConstructionScript`)